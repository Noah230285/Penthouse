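; Player examination component that adds a background blur and applies controller freeze flags when the player enters the examine state.
; Enter and exit extend the parent logic, re-seed the blur value from its eased result and flip the blur direction.
; Tick ramps that value between zero and one, applies direction-dependent cubic easing and writes BlurStrength to the post-processing Material Parameter Collection.
; Exit clears no freeze flags here.
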(event EventBeginPlay)

(event EventTick
  (params (DeltaSeconds :type Float%20%28single-precision%29))
  (Variables|Default|SetCurrentBlurValue (Math|Float|Clamp(Float) (+ (* DeltaSeconds (Math|Float|SelectFloat 1.0 -1.0 (Variables|Default|GetBluring))) (Variables|Default|GetCurrentBlurValue))))
  (bind _modified (CallFunction|BlurLerptoSmoothed))
  (Rendering|Material|SetScalarParameterValue "/Game/Shaders/PostProcessing/MP_PostProcessing.MP_PostProcessing" "BlurStrength" _modified :!class /Script/Engine.KismetMaterialLibrary))

(event EventEnterExamineState
  (params (ActorClass :type Examinable%20Object%20Actor%20Class%20Reference))
  (|CallParentFunction ActorClass)
  (Utilities|FlowControl|Sequence
    (:then_0
      (bind _modified (CallFunction|BlurLerptoSmoothed))
      (Variables|Default|SetCurrentBlurValue _modified)
      (Variables|Default|SetBluring true))
    (:then_1
      (bind _asbp_first_person_player_controller (Utilities|Casting|CastToBP_FirstPersonPlayerController (Game|GetPlayerController 0)))
      (Class|PenthousePlayerController|ApplyFreezeFlags _asbp_first_person_player_controller (Math|Conversions|ToByte(Integer) (|BitmaskLiteral 1))))))

(event EventExitExamineState
  (|CallParentFunction)
  (bind _modified (CallFunction|BlurLerptoSmoothed))
  (Variables|Default|SetCurrentBlurValue _modified)
  (Variables|Default|SetBluring false))

(event EventAddExamineActor
  (params (ActorClass :type Examinable%20Object%20Actor%20Class%20Reference))
  (|CallParentFunction ActorClass))

(event EventRemoveExamineActor
  (|CallParentFunction))

(fn BlurLerptoSmoothed
  (bind _currentblurvalue (Variables|Default|GetCurrentBlurValue))
  (return (Math|Float|SelectFloat (+ (Math|Float|Power (- _currentblurvalue 1.0) 3.0) 1.0) (Math|Float|Power _currentblurvalue 3.0) (Variables|Default|GetBluring))))