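; SC_PlayerInteractor is a player component, apparently an unfinished stub for interacting with the world from BP_FirstPersonCharacter.
; BeginPlay casts its owner to that character and caches it.
; The IA_Interact input only casts the owner to Character, and Tick only checks that the cached owner is valid.
; A single line trace by profile and a camera location lookup exist but are not connected, so no interaction happens yet.
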(event Input|EnhancedActionEvents|EnhancedInputActionIA_Interact
  (params (ActionValue :type Boolean) (ElapsedSeconds :type Float%20%28double-precision%29) (TriggeredSeconds :type Float%20%28double-precision%29) (InputAction :type Input%20Action%20Object%20Reference :default "/Game/Input/Actions/IA_Interact.IA_Interact"))
  (Utilities|Casting|CastToCharacter (Components|GetOwner)))

(event EventTick
  (params (DeltaSeconds :type Float%20%28single-precision%29))
  (Utilities|IsValid (Variables|Default|GetOwner)))

(event EventBeginPlay
  (bind _asbp_first_person_character (Utilities|Casting|CastToBP_FirstPersonCharacter (Components|GetOwner)))
  (Variables|Default|SetOwner _asbp_first_person_character))