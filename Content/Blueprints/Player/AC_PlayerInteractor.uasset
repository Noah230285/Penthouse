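; Player interaction component for the first-person character that lets the player use InteractableTrigger actors in view.
; On BeginPlay it caches its owning BP_FirstPersonCharacter.
; Each tick it sphere-traces on the Visibility channel forward from the first-person camera, storing a hit InteractableTrigger as the hovered target and clearing it otherwise.
; The IA_Interact input calls OnInteracted on that target, passing the owning character.
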(event Input|EnhancedActionEvents|EnhancedInputActionIA_Interact
  (params (ActionValue :type Boolean) (ElapsedSeconds :type Float%20%28double-precision%29) (TriggeredSeconds :type Float%20%28double-precision%29) (InputAction :type Input%20Action%20Object%20Reference :default "/Game/Input/Actions/IA_Interact.IA_Interact"))
  (bind _hoveredinteractable (Variables|Default|GetHoveredInteractable))
  (Utilities|IsValid _hoveredinteractable
    (:Is%20Valid
      (Class|InteractableTrigger|OnInteracted _hoveredinteractable (Variables|Default|GetOwner)))))

(event EventTick
  (params (DeltaSeconds :type Float%20%28single-precision%29))
  (bind _owner (Variables|Default|GetOwner))
  (bind _firstpersoncameracomponent (Variables|/Script/Penthouse.PenthouseCharacter|GetFirstPersonCameraComponent _owner))
  (bind _returnvalue (Transformation|GetWorldLocation _firstpersoncameracomponent))
  (Utilities|IsValid _owner
    (:Is%20Valid
      (bind (_outhit _returnvalue_2) (Collision|SphereTraceByChannel _returnvalue (+ _returnvalue (* (Math|Vector|GetForwardVector _firstpersoncameracomponent) (Variables|Default|GetIntreractLength))) (Variables|Default|GetIntreractRadius) "TraceTypeQuery1" false 0 "None"))
      (if _returnvalue_2
        (bind _asinteractable_trigger (Utilities|Casting|CastToInteractableTrigger (.HitActor (Collision|BreakHitResult _outhit)))
          (:then
            (Variables|Default|SetHoveredInteractable _asinteractable_trigger))
          (:CastFailed
            (Variables|Default|SetHoveredInteractable 0 :!label _label)))
        (else
          (goto _label))))))

(event EventBeginPlay
  (bind _asbp_first_person_character (Utilities|Casting|CastToBP_FirstPersonCharacter (Components|GetOwner)))
  (Variables|Default|SetOwner _asbp_first_person_character))